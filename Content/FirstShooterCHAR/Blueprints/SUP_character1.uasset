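; Supporting NPC character for a first-person shooter that approaches a sighted player to deliver dialogue.
; PawnSensing drives SensorCollider, which moves toward the player unless health is low, cycles one of two speech arrays, and pauses for mission-choice widgets at set lines.
; Capsule overlaps use actor tags to handle ammo, health pickups and firearm damage.
; The random-destination patrol is an empty stub, with its waypoint movement left disconnected.
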(event `self.CapsuleComponent.OnComponentBeginOverlap`
  (params (OverlappedComponent :type "PrimitiveComponent Object Reference") (OtherActor :type "Actor Object Reference") (OtherComp :type "PrimitiveComponent Object Reference") (OtherBodyIndex :type Integer) (bFromSweep :type Boolean) (SweepResult :type "HitResult Structure (by ref)"))
  ; Collider
  (if (`self.ActorHasTag` OtherActor "Amm")
    (`KismetSystemLibrary.PrintString` "Ammunition logic")
    (`self.AddAmm`)
    (if (>= (`self.CurrentEnemyAmm`) 6.0)
      (`KismetSystemLibrary.PrintString` "AmmunitionFull"))
    (`self.K2_DestroyActor` OtherActor)
    (elif (`self.ActorHasTag` OtherActor "HealthEN")
      (if (< (`self.CurrentHP`) 75.0)
        (`self.Health`))
      (elif (`self.ActorHasTag` OtherActor "SECfirearm")
        _
        (elif (`self.ActorHasTag` OtherActor "DefaultFirearm")
          (`self.K2_DestroyActor` OtherActor)
          (`/Game/Blueprints/CHAR_Moves.CHARDamagedHealth_1`)
          (elif (`self.ActorHasTag` OtherActor "SecondFirearm")
            (`self.K2_DestroyActor` OtherActor)
            (`/Game/Blueprints/CHAR_Moves.CHARDamagedHealth_2`)))))))

(event `SensorCollider`
  ; Character Movement
  (if (== (`self.See Player?`) true)
    (`MovementComponent.StopMovementImmediately` (`self.CharacterMovement`))
    (`self.StopSprinting`)
    (`|AIMoveTo` self (0.0 0.0 0.0) (`GameplayStatics.GetPlayerController` 0) 1000.0
      (:`then`
        _)
      (:`OnSuccess`
        _))
    (`KismetSystemLibrary.Delay` 2.0)
    (`/Game/Blueprints/DialogueInterface.DialogueCentre`)
    (if (== (`self.TalkingIndex_1`) 8)
      (bind _returnvalue (`|CreateWidget` "/Game/UI/Widgets/ChoiceMissionTEAM1.ChoiceMissionTEAM1_C"))
      (`UserWidget.AddToViewport` _returnvalue 0)
      (`GameplayStatics.SetGamePaused` true)
      (set `self.TalkingIndex_1` 0)
      (set `self.DialogueSetSwitch_` 2)
      (else
        (`self.StopSprinting`)
        (`KismetSystemLibrary.Delay` 4.0)
        (set `self.See Player?` false)
        (`self.SensorCollider`)
        (if (== (`self.DialogueSetSwitch_`) 2)
          (if (== (`self.TalkingIndex`) 6)
            (`GameplayStatics.SetGamePaused` true)
            (bind _returnvalue_2 (`|CreateWidget` "/Game/UI/Widgets/ChoiceMission_timeTEAM.ChoiceMission_timeTEAM_C"))
            (`UserWidget.AddToViewport` _returnvalue_2 0)))))
    (else
      (`/Game/Blueprints/CHAR_Moves.SetRandomDestinations`))))

(event `self.PawnSensing.OnSeePawn`
  (params (Pawn :type "Pawn Object Reference"))
  ; Sensors
  (if (`self.ActorHasTag` Pawn "Player")
    (if (< (`self.DefaultHP`) 25.0)
      (set `self.See Player?` false)
      (else
        (set `self.See Player?` true)))
    (`self.SensorCollider`)
    (else
      (`KismetSystemLibrary.PrintString` "not player"))))

(event `self.ReceiveBeginPlay`
  ; Start
  (if (not (> (`self.CurrentPath`) 0))
    (`self.SensorCollider`)))

(event `self.SpawnPointersActors`
  ; Spawn
  (bind _outactors (`GameplayStatics.GetAllActorsOfClass` "/Game/Blueprints/BP_WaypointsRandom1.BP_WaypointsRandom1_C"))
  (bind _outitem (`KismetArrayLibrary.Array_Random` _outactors))
  (`self.K2_SetActorLocation` (`self.K2_GetActorLocation` _outitem))
  (set `self.DefaultHP` 100.0)
  (`self.SensorCollider`))

(event `self.SetRandomDestinations`
  ; Waypoints
)

(event `self.DialogueCentre`
  ; Dialogue
  (if (== (`self.DialogueSetSwitch_`) 2)
    (if (<= (`self.TalkingIndex`) (`KismetArrayLibrary.Array_Length` (`self.DialogueSpeech_1`))) :!label _label
      (`self.DisplayDialogue`
        (:`then`
          (`TextBlock.SetText` (`/Game/UI/Widgets/Dialogue.Dialogue_TXT` (`self.DisplayDialogue`)) (`KismetTextLibrary.Conv_StringToText` (`|GetArrayItem` (`self.DialogueSpeech_1`) (`self.TalkingIndex`))))
          (`/Engine/EditorBlueprintResources/StandardMacros.IncrementInt` (`self.TalkingIndex`)))
        (:`else`
          (bind _returnvalue (`|CreateWidget` "/Game/UI/Widgets/Dialogue.Dialogue_C" (`GameplayStatics.GetPlayerController` 0)))
          (bind _output_get (set `self.DisplayDialogue` _returnvalue))
          (`UserWidget.AddToViewport` _output_get 0)))
      (else
        (set `self.TalkingIndex` 0)
        (goto _label)))
    (elif (== (`self.DialogueSetSwitch_`) 1)
      (if (<= (`self.TalkingIndex_1`) (`KismetArrayLibrary.Array_Length` (`self.MARKDialogueSpeech`))) :!label _label_2
        (`self.DisplayDialogue`
          (:`then`
            (`TextBlock.SetText` (`/Game/UI/Widgets/Dialogue.Dialogue_TXT` (`self.DisplayDialogue`)) (`KismetTextLibrary.Conv_StringToText` (`|GetArrayItem` (`self.MARKDialogueSpeech`) (`self.TalkingIndex_1`))))
            (`/Engine/EditorBlueprintResources/StandardMacros.IncrementInt` (`self.TalkingIndex_1`)))
          (:`else`
            (bind _returnvalue_2 (`|CreateWidget` "/Game/UI/Widgets/Dialogue.Dialogue_C" (`GameplayStatics.GetPlayerController` 0)))
            (bind _output_get_2 (set `self.DisplayDialogue` _returnvalue_2))
            (`UserWidget.AddToViewport` _output_get_2 0)))
        (else
          (set `self.TalkingIndex_1` 0)
          (goto _label_2))))))

(fn `AddAmm`
  (bind _output_get (set `self.CurrentEnemyAmm` (`KismetMathLibrary.FClamp` (+ (`self.CurrentEnemyAmm`) (`self.AddEnemyAmm`)) 0.0 (`self.FullEnemyAmm`))))
  (`KismetSystemLibrary.PrintString` (`KismetStringLibrary.Conv_DoubleToString` _output_get)))

(fn `ForwardMovement`
  (bind (_returnvalue_roll _returnvalue_pitch _returnvalue_yaw) (`KismetMathLibrary.BreakRotator` (`self.GetControlRotation`)))
  (`self.AddMovementInput` (`KismetMathLibrary.GetForwardVector` (`KismetMathLibrary.MakeRotator` _returnvalue_roll 0.0 _returnvalue_yaw))))

(fn `Health`
  (bind _output_get (set `self.DefaultHP` (`KismetMathLibrary.FClamp` (+ (`self.DefaultHP`) (`self.AddedHP`)) 0.0 (`self.MaxHP`))))
  (if (>= (`self.DefaultHP`) 100.0)
    (`KismetSystemLibrary.PrintString` "healthfull")
    (else
      (`KismetSystemLibrary.PrintString` (`KismetStringLibrary.Conv_DoubleToString` _output_get) true true (struct :`G` 1.0 :`B` 0.056098 :`A` 1.0)))))

(fn `MinusAmm`
  (bind _output_get (set `self.CurrentEnemyAmm` (`KismetMathLibrary.FClamp` (- (`self.CurrentEnemyAmm`) (`self.MinusEnemyAmm`)) 0.0 (`self.FullEnemyAmm`))))
  (`KismetSystemLibrary.PrintString` (`KismetStringLibrary.Conv_DoubleToString` _output_get) true true (struct :`R` 1.0 :`B` 0.137026 :`A` 1.0)))

(fn `RightMovement`
  (bind (_returnvalue_roll _returnvalue_pitch _returnvalue_yaw) (`KismetMathLibrary.BreakRotator` (`self.GetControlRotation`)))
  (`self.AddMovementInput` (`KismetMathLibrary.GetRightVector` (`KismetMathLibrary.MakeRotator` _returnvalue_roll 0.0 _returnvalue_yaw))))

(fn `Sprinting`
  (set `CharacterMovementComponent.MaxWalkSpeed` (`self.RunSpeed`) (`self.CharacterMovement`)))

(fn `StopSprinting`
  (set `CharacterMovementComponent.MaxWalkSpeed` (`self.WalkSpeed`) (`self.CharacterMovement`)))

(fn `UserConstructionScript`)